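; GA_Charm_EmberHeart is the ability for the Ember Heart charm, granting bonus max health and applying burns.
; A stat tag stack count sets the max health effect's SetByCaller magnitude, and an update event removes and reapplies it through its stored handle.
; Gameplay message listeners apply the burn effect to target data received on the Burn channel.
; The Explosion channel listener has no response wired, and activation prints a debug string.
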(event `self.K2_ActivateAbility`
  (`parent.K2_ActivateAbility`)
  (add `self.OnTagStacksChanged` (`|CreateDelegate` :!event `UpdateMaxHealth_GE`))
  (`self.ListenEvents`)
  (`KismetSystemLibrary.PrintString` (`KismetSystemLibrary.Conv_PrimaryAssetTypeToString` (`.PrimaryAssetType` (break `PrimaryAssetId` (`KismetSystemLibrary.GetPrimaryAssetIdFromObject` self))))))

(event `self.PostInitStatTagStack`
  (`self.ApplyMaxHealth_GE`))

(event `self.K2_OnEndAbility`
  (params (bWasCancelled :type Boolean))
  (`parent.K2_OnEndAbility` bWasCancelled))

(event `ApplyMaxHealth_GE`
  (bind _returnvalue (`AbilitySystemBlueprintLibrary.AssignTagSetByCallerMagnitude` (`self.MakeOutgoingGameplayEffectSpec` (`self.BaseEffectClass`)) (struct :`TagName` "SetByCaller.Magnitude") (`KismetMathLibrary.Conv_IntToDouble` (`self.GetStatTagStackCount` (struct :`TagName` "CharmAbility.EmberHeart.MaxHealthIncrease")))))
  (bind _returnvalue_2 (`self.K2_ApplyGameplayEffectSpecToOwner` _returnvalue))
  (set `self.MaxHP_EffectHandle` _returnvalue_2))

(event `UpdateMaxHealth_GE`
  (bind _maxhp_effecthandle (`self.MaxHP_EffectHandle`))
  (`self.BP_RemoveGameplayEffectFromOwnerWithHandle` _maxhp_effecthandle)
  (`AbilityTask_WaitGameplayEffectRemoved.WaitForGameplayEffectRemoved` _maxhp_effecthandle
    (:`OnRemoved`
      (`self.ApplyMaxHealth_GE`))))

(event `ListenEvents`
  (`|ExecutionSequence`
    (:`then_0`
      (bind (_asynctaskproxy _actualchannel _payload) (`|AsyncAction_ListenForGameplayMessages` (struct :`TagName` "GameplayAbilityEvent.EmberHeart.Burn") "/Script/GameplayAbilities.GameplayAbilityTargetDataHandle")
        (:`OnMessageReceived`
          (`self.BP_ApplyGameplayEffectToTarget` _payload (`self.GE_EmberHeart_Burn`)))))
    (:`then_1`
      (`|AsyncAction_ListenForGameplayMessages` (struct :`TagName` "GameplayAbilityEvent.EmberHeart.Explosion") "/Script/GameplayAbilities.GameplayAbilityTargetDataHandle"))))