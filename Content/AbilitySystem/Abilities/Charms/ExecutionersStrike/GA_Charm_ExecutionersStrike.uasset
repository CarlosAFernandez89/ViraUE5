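; Charm gameplay ability that gives a chance to instantly execute low-health enemies.
; On activation it listens for ExecutionersStrike gameplay messages carrying the enemy's health percentage, type and ability system component.
; Each enemy tier (Normal, Elite, Boss, Archboss) has its own health threshold, with a shared random execution chance.
; A successful roll triggers the death ability directly on the enemy's ASC.
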(event `self.K2_ActivateAbility`
  (`parent.K2_ActivateAbility`)
  (`self.ListenEvents`))

(event `self.K2_OnEndAbility`
  (params (bWasCancelled :type Boolean))
  (`parent.K2_OnEndAbility` bWasCancelled))

(event `ListenEvents`
  (bind _health_percentage (`self.Health Percentage`))
  (bind _returnvalue (< (`KismetMathLibrary.RandomFloatInRange` 0.0 1.0) (`self.ExecutionChance`)))
  (bind (_asynctaskproxy _actualchannel _payload) (`|AsyncAction_ListenForGameplayMessages` (struct :`TagName` "GameplayAbilityEvent.ExecutionersStrike") "/Game/AbilitySystem/Abilities/Charms/ExecutionersStrike/Struct_ExecutionersStrike_Data.Struct_ExecutionersStrike_Data")
    (:`OnMessageReceived`
      (bind (_enemyasc _enemytype _healthpercentage) (break `/Game/AbilitySystem/Abilities/Charms/ExecutionersStrike/Struct_ExecutionersStrike_Data` _payload))
      (set `self.Health Percentage` _healthpercentage)
      (switch `EVyraEnemyType` _enemytype
        (:`NORMAL`
          (if (and (<= _health_percentage (`self.NormalHealthThreshold`)) _returnvalue)
            (`AbilitySystemComponent.TryActivateAbilityByClass` _enemyasc "/Game/AbilitySystem/Abilities/Enemies/GA_Enemy_Death.GA_Enemy_Death_C" true :!label _label)))
        (:`ELITE`
          (if (and (<= _health_percentage (`self.EliteHealthThreshold`)) _returnvalue)
            (goto _label)))
        (:`BOSS`
          (if (and (<= _health_percentage (`self.BossHealthThreshold`)) _returnvalue)
            (goto _label)))
        (:`ARCHBOSS`
          (if (and (<= _health_percentage (`self.ArchBossHealthThreshold`)) _returnvalue)
            (goto _label)))))))