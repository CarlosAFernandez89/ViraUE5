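; Gameplay ability for the Embers Echo charm that spawns projectiles in response to gameplay messages.
; On activation it listens on the EmbersEcho and EmbersEcho.Hit channels, each carrying a transform as payload.
; Each message spawns a tag-stack count of projectiles at jittered points around that transform, randomly scaled and oriented toward the avatar's location, passing along damage parameters.
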(event `self.K2_ActivateAbility`
  (`parent.K2_ActivateAbility`)
  (`self.ListenEvents`))

(event `self.K2_OnEndAbility`
  (params (bWasCancelled :type Boolean))
  (`parent.K2_OnEndAbility` bWasCancelled))

(event `ListenEvents`
  (`|ExecutionSequence`
    (:`then_0`
      (bind (_asynctaskproxy _actualchannel _payload) (`|AsyncAction_ListenForGameplayMessages` (struct :`TagName` "CharmAbility.EmbersEcho") "/Script/CoreUObject.Transform")
        (:`OnMessageReceived`
          (`self.SpawnProjectiles` _payload))))
    (:`then_1`
      (bind (_asynctaskproxy_2 _actualchannel_2 _payload_2) (`|AsyncAction_ListenForGameplayMessages` (struct :`TagName` "CharmAbility.EmbersEcho.Hit") "/Script/CoreUObject.Transform")
        (:`OnMessageReceived`
          (`self.SpawnProjectiles` _payload_2))))))

(fn `GetRandomScale`
  (params (Min :type "Float (double-precision)") (Max :type "Float (double-precision)"))
  (returns (RandomVectorInRange :type "Vector Structure"))
  (bind _returnvalue (`KismetMathLibrary.RandomFloatInRange` Min Max))
  (return (`KismetMathLibrary.MakeVector` _returnvalue _returnvalue _returnvalue)))

(fn `SpawnProjectiles`
  (params (InTransform :type "Transform Structure (by ref)"))
  (bind _location (.location InTransform))
  (for _ (range (`self.GetStatTagStackCount` (struct :`TagName` "CharmAbility.EmbersEcho.ProjectileCount")))
    (`|SpawnActorFromClass` "/Game/AbilitySystem/Abilities/Charms/EmbersEcho/B_Charm_EmbersEcho_Projectile.B_Charm_EmbersEcho_Projectile_C" (`KismetMathLibrary.MakeTransform` (`KismetMathLibrary.RandomPointInBoundingBox` _location (10.0 25.0 25.0)) (`KismetMathLibrary.MakeRotFromX` (- (`Actor.K2_GetActorLocation` (`self.GetAvatarActorFromActorInfo`)) _location)) (`self.GetRandomScale` 0.2 0.5)) "AdjustIfPossibleButAlwaysSpawn" "MultiplyWithRoot" (`self.GetAvatarActorFromActorInfo`) (`self.GE Damage`) (`self.Extra Damage`) false null)))