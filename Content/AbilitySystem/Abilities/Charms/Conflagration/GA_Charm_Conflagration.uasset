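; Gameplay ability for the Conflagration charm that deals explosion damage to enemy characters around a reported location.
; On activation it listens for Conflagration Explode gameplay messages, using the Transform payload as the center of a sphere overlap for enemy pawns, ignoring the avatar.
; Radius and damage come from stat tag stacks, with damage negated and applied to all hit actors through a SetByCaller gameplay effect.
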(event `self.K2_ActivateAbility`
  (`parent.K2_ActivateAbility`)
  (`self.ListenEvents`))

(event `ListenEvents`
  (bind (_asynctaskproxy _actualchannel _payload) (`|AsyncAction_ListenForGameplayMessages` (struct :`TagName` "GameplayAbilityEvent.Conflagration.Explode") "/Script/CoreUObject.Transform")
    (:`OnMessageReceived`
      (bind (_outactors _returnvalue) (`KismetSystemLibrary.SphereOverlapActors` (.location _payload) (`KismetMathLibrary.Conv_IntToDouble` (`self.GetStatTagStackCount` (struct :`TagName` "CharmAbility.Conflagration.ExplosionRadius"))) (`|MakeArray` "ObjectTypeQuery3" :!type "EObjectTypeQuery Enum") "/Script/Vira.VyraEnemyCharacter" (`|MakeArray` (`self.GetAvatarActorFromActorInfo`))))
      (if _returnvalue
        (bind _returnvalue_2 (`AbilitySystemBlueprintLibrary.AssignTagSetByCallerMagnitude` (`self.MakeOutgoingGameplayEffectSpec` (`self.GE_Conflagration_Damage`)) (struct :`TagName` "SetByCaller.Damage") (`KismetMathLibrary.Conv_IntToDouble` (* (`self.GetStatTagStackCount` (struct :`TagName` "CharmAbility.Conflagration.Damage")) -1))))
        (`self.K2_ApplyGameplayEffectSpecToTarget` _returnvalue_2 (`AbilitySystemBlueprintLibrary.AbilityTargetDataFromActorArray` _outactors))))))