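; Charm gameplay ability that lets Vyra cheat death, reviving her with a percentage of maximum health.
; When triggered by a gameplay event, it commits, applies a heal effect to itself through a SetByCaller magnitude, then ends.
; The HealthRestored stat tag stack count sets the percentage and feeds the charm's description, which refreshes whenever tag stacks change.
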(event `self.K2_ActivateAbilityFromEvent`
  (params (EventData :type "GameplayEventData Structure (by ref)"))
  (bind _returnvalue (`self.GetAvatarActorFromActorInfo`))
  (bind _returnvalue_2 (`self.K2_CommitAbility`))
  (if _returnvalue_2
    (bind _returnvalue_3 (`AbilitySystemBlueprintLibrary.MakeSpecHandleByClass` (`self.EffectClass`) _returnvalue _returnvalue))
    (bind _returnvalue_4 (`AbilitySystemBlueprintLibrary.AssignTagSetByCallerMagnitude` _returnvalue_3 (struct :`TagName` "SetByCaller.Heal") (* (`GSCCoreComponent.GetMaxHealth` (`self.GetVyraGSCCoreComponent`)) (/ (`KismetMathLibrary.Conv_IntToDouble` (`self.GetStatTagStackCount` (struct :`TagName` "CharmAbility.CheatDeath.HealthRestored"))) 100.0))))
    (`AbilitySystemComponent.BP_ApplyGameplayEffectSpecToSelf` (`self.GetAbilitySystemComponentFromActorInfo`) _returnvalue_4)
    (`self.K2_EndAbility`)
    (else
      (`self.K2_EndAbility`))))

(event `self.OnTagStacksChangedEvent`
  (`parent.OnTagStacksChangedEvent`)
  (`self.UpdateCharmInformation`))

(event `UpdateCharmInformation`
  (bind (_name _description _cost) (break `CharmAbilityInformation` (`self.CharmAbilityInformation`)))
  ;[0.02519 0.02217 0.02029] Update Charm information
  (set `self.CharmAbilityInformation` (make `CharmAbilityInformation` _name (`|FormatText` "Upon death, Vyra consumes her remaining internal fire to Cheat Death, reviving with {Percentage}% of her maximum health." (`self.GetStatTagStackCount` (struct :`TagName` "CharmAbility.CheatDeath.HealthRestored"))) _cost)))

(fn `K2_ShouldAbilityRespondToEvent`
  (params (ActorInfo :type "GameplayAbilityActorInfo Structure") (Payload :type "GameplayEventData Structure"))
  (returns (ReturnValue :type Boolean))
  (return true))