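; Gameplay ability for the Soul Reaper arcade passive, applying its gameplay effect to the owner on activation.
; The effect spec uses the ability's level, and its active handle is stored after application.
; When the avatar receives the Soul Reaper gameplay event, the stored effect is removed and reapplied at a fixed level 3 instead of the ability's level.
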(event `self.K2_ActivateAbility`
  (`parent.K2_ActivateAbility`)
  (bind _returnvalue (`self.K2_ApplyGameplayEffectSpecToOwner` (`self.MakeOutgoingGameplayEffectSpec` "/Game/AbilitySystem/Abilities/Arcade/Passive/SoulReaper/GE_ArcadePassive_SoulReaper.GE_ArcadePassive_SoulReaper_C" (`KismetMathLibrary.Conv_IntToDouble` (`self.GetAbilityLevel`)))))
  (set `self.ActiveGameplayEffectHandle` _returnvalue)
  (`AbilityAsync_WaitGameplayEvent.WaitGameplayEventToActor` (`self.GetAvatarActorFromActorInfo`) (struct :`TagName` "GameplayAbilityEvent.Arcade.Passive.SoulReaper")
    (:`EventReceived`
      (`self.BP_RemoveGameplayEffectFromOwnerWithHandle` (`self.ActiveGameplayEffectHandle`))
      (bind _returnvalue_2 (`self.K2_ApplyGameplayEffectSpecToOwner` (`self.MakeOutgoingGameplayEffectSpec` "/Game/AbilitySystem/Abilities/Arcade/Passive/SoulReaper/GE_ArcadePassive_SoulReaper.GE_ArcadePassive_SoulReaper_C" 3.0)))
      (set `self.ActiveGameplayEffectHandle` _returnvalue_2))))