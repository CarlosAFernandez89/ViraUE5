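; Gameplay ability for the Crimson Claws arcade attack, dealing damage when its animation registers a combat collision.
; Activation plays a montage at a rate read from an avatar attribute, falling back to 1.0 if that attribute is not found.
; Each collision gameplay event applies the damage effect to the event's target data, and the ability ends when the montage completes, blends out, is interrupted or is cancelled.
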(event `self.K2_ActivateAbility`
  (`parent.K2_ActivateAbility`)
  (bind (_asynctaskproxy _eventtag _eventdata) (`GSCTask_PlayMontageWaitForEvent.PlayMontageAndWaitForEvent` "None" (`self.Montage to Play`) (struct :`GameplayTags` (struct :`(TagName` "Event.Combat.Attack.Collision"))) (`self.GetAttackSpeed`))
    (:`OnCompleted`
      (`self.K2_EndAbility` :!label _label))
    (:`OnBlendOut`
      (goto _label))
    (:`OnInterrupted`
      (goto _label))
    (:`OnCancelled`
      (goto _label))
    (:`EventReceived`
      (`|SwitchGameplayTag` _eventtag
        (:`Event.Combat.Attack.Collision`
          (`|ExecutionSequence`
            (:`then_0`
              (bind _returnvalue (`self.BP_ApplyGameplayEffectToTarget` (`.TargetData` (break `GameplayEventData` _eventdata)) (`self.GEDamage`)))
              (for _ _returnvalue
                _))))))))

(fn `GetAttackSpeed`
  (returns (ReturnValue :type "Float (double-precision)"))
  (bind (_bsuccessfullyfoundattribute _returnvalue) (`AbilitySystemBlueprintLibrary.GetFloatAttribute` (`self.GetAvatarActorFromActorInfo`) (struct :`AttributeName` "AttackSpeed" :`Attribute` "/Script/Vira.CombatAttributeSet:AttackSpeed" :`AttributeOwner` "/Script/CoreUObject.Class'/Script/Vira.CombatAttributeSet'")))
  (return (`KismetMathLibrary.SelectFloat` _returnvalue 1.0 _bsuccessfullyfoundattribute)))