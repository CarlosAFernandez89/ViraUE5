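; Gameplay ability for the Arcade Crimson Claws active attack, a melee strike that damages targets and restores the owner's mana.
; On activation it runs the parent logic, then plays an attack montage scaled by attack speed and listens for collision events.
; Each collision event applies the damage effect to its target data, then grants the owner one melee mana-regain stack per applied effect.
; The ability ends when the montage completes, blends out, or is interrupted or cancelled.
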(event `self.K2_ActivateAbility`
  (`parent.K2_ActivateAbility`)
  (bind (_asynctaskproxy _eventtag _eventdata) (`GSCTask_PlayMontageWaitForEvent.PlayMontageAndWaitForEvent` "None" (`self.Montage to Play`) (struct :`GameplayTags` (struct :`(TagName` "Event.Combat.Attack.Collision"))) (`self.GetAttackSpeed`))
    (:`OnCompleted`
      (`self.K2_EndAbility` :!label _label))
    (:`OnBlendOut`
      (goto _label))
    (:`OnInterrupted`
      (goto _label))
    (:`OnCancelled`
      (goto _label))
    (:`EventReceived`
      (`|SwitchGameplayTag` _eventtag
        (:`Event.Combat.Attack.Collision`
          (`|ExecutionSequence`
            (:`then_0`
              (bind _returnvalue (`self.BP_ApplyGameplayEffectToTarget` (`.TargetData` (break `GameplayEventData` _eventdata)) (`self.GEDamage`) (`self.GetAbilityLevel`)))
              (for _ _returnvalue
                (`self.BP_ApplyGameplayEffectToOwner` "/Game/AbilitySystem/Abilities/Player/Attacks/GE_Player_Melee_ManaRegain.GE_Player_Melee_ManaRegain_C" (`self.GetAbilityLevel`))))))))))