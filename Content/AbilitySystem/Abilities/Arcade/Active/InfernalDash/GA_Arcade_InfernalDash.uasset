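; Gameplay ability for the Arcade active Infernal Dash, a cast-time move that teleports when the cast succeeds.
; Casting start plays a montage at cast speed, and the ability ends when it completes, blends out, is interrupted or is cancelled.
; Interruption or cancellation also broadcasts a cast-failed UI message through the Gameplay Message Subsystem.
; Casting success calls PerformTeleport, which is not defined in this graph.
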(event `self.K2_ActivateAbility`
  (`parent.K2_ActivateAbility`))

(event `self.OnCastingStarted`
  (`parent.OnCastingStarted`)
  (`GSCTask_PlayMontageWaitForEvent.PlayMontageAndWaitForEvent` "None" (`self.MontageToPlay`) (struct) (`self.GetCastSpeed`)
    (:`OnCompleted`
      (`self.K2_EndAbility` :!label _label))
    (:`OnBlendOut`
      (goto _label))
    (:`OnInterrupted`
      (`self.K2_EndAbility` :!label _label_2)
      (`GameplayMessageSubsystem.K2_BroadcastMessage` (subsystem `GameplayMessageSubsystem`) (struct :`TagName` "UIMessaging.Ability.Cast.Failed") (make `VyraCastTimeMessage` "" 1.0)))
    (:`OnCancelled`
      (goto _label_2))))

(event `self.OnCastingSucceeded`
  (`parent.OnCastingSucceeded`)
  (`self.PerformTeleport`))