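; Active Arcade gameplay ability Blood Scythe: a melee-style cone attack that damages targets and heals the owner for each one hit.
; It plays a montage scaled by attack speed and ends when the montage finishes, blends out or is stopped.
; On the montage trigger event, a cone trace feeds a level-scaled damage effect.
; Each returned effect handle reapplies a fixed SetByCaller heal spec to the owner.
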(event `self.K2_ActivateAbility`
  (`parent.K2_ActivateAbility`)
  (bind (_asynctaskproxy _eventtag) (`GSCTask_PlayMontageWaitForEvent.PlayMontageAndWaitForEvent` "None" (`self.Montage to Play`) (struct :`GameplayTags` (struct :`(TagName` "Event.Montage.Trigger"))) (`self.GetAttackSpeed`))
    (:`OnCompleted`
      (`self.K2_EndAbility` :!label _label))
    (:`OnBlendOut`
      (goto _label))
    (:`OnInterrupted`
      (goto _label))
    (:`OnCancelled`
      (goto _label))
    (:`EventReceived`
      (`|SwitchGameplayTag` _eventtag
        (:`Event.Montage.Trigger`
          (bind (_outhits _returnvalue) (`self.PerformConeTrace`))
          (bind _returnvalue_2 (`self.K2_ApplyGameplayEffectSpecToTarget` (`self.MakeOutgoingGameplayEffectSpec` (`self.GE_Damage`) (`KismetMathLibrary.Conv_IntToDouble` (`self.GetAbilityLevel`))) _returnvalue))
          ;[1 0 0] Regain Life for every enemy that was hit.
          (bind _returnvalue_3 (`AbilitySystemBlueprintLibrary.AssignTagSetByCallerMagnitude` (`self.MakeOutgoingGameplayEffectSpec` (`self.GE_OnHitRegen`) (`KismetMathLibrary.Conv_IntToDouble` (`self.GetAbilityLevel`))) (struct :`TagName` "SetByCaller.Heal") 2.0))
          (set `self.OnHitHeal_EffectSpec` _returnvalue_3)
          (for _ _returnvalue_2
            (`self.K2_ApplyGameplayEffectSpecToOwner` (`self.OnHitHeal_EffectSpec`))))))))