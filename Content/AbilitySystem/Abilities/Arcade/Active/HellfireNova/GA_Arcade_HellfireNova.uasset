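; Arcade channelled ability Hellfire Nova, which spawns a damaging B_HellfireNova_Collider at the avatar when the parent class reports a normal or perfect channel.
; Perfect channelling passes a higher-level damage effect spec than normal channelling.
; Gameplay tag stack counts set the collider's max radius and optional interval damage.
; Activation plays a cast-speed-scaled montage that ends the ability, broadcasting a channelling UI message on cancel or event received.
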(event `self.StartChannelling`
  (`parent.StartChannelling`))

(event `self.OnChannellingComplete`
  (params (TotalChannelTime :type "Float (single-precision)"))
  (`parent.OnChannellingComplete` TotalChannelTime))

(event `self.K2_ActivateAbility`
  (`parent.K2_ActivateAbility`)
  (`GSCTask_PlayMontageWaitForEvent.PlayMontageAndWaitForEvent` "None" (`self.MontageToPlay`) (struct) (`self.GetCastSpeed`)
    (:`OnCompleted`
      (`self.K2_EndAbility` :!label _label))
    (:`OnBlendOut`
      (goto _label))
    (:`OnCancelled`
      (`self.K2_EndAbility` :!label _label_2)
      (`GameplayMessageSubsystem.K2_BroadcastMessage` (subsystem `GameplayMessageSubsystem`) (struct :`TagName` "UIMessaging.Ability.Channelling") (make `VyraChannelingMessage_Released` false)))
    (:`EventReceived`
      (goto _label_2))))

(event `self.OnPerfectChannelling`
  (params (TotalChannelTime :type "Float (single-precision)"))
  (bind _returnvalue (`self.GetAvatarActorFromActorInfo`))
  (bind _returnvalue_2 (`VyraBlueprintFunctionLibrary.GetVyraAbilitySystemComponent`))
  (`parent.OnPerfectChannelling` TotalChannelTime)
  (`|SpawnActorFromClass` "/Game/AbilitySystem/Abilities/Arcade/Active/HellfireNova/B_HellfireNova_Collider.B_HellfireNova_Collider_C" (`Actor.GetTransform` _returnvalue) "AlwaysSpawn" "MultiplyWithRoot" _returnvalue 1.0 (`VyraAbilitySystemComponent.GetGameplayTagStackCount` _returnvalue_2 (struct :`TagName` "GameplayTagStack.Arcade.Active.HellfireNova.MaxRadius")) 5.0 (`KismetMathLibrary.Conv_IntToBool` (`KismetMathLibrary.FFloor` (`VyraAbilitySystemComponent.GetGameplayTagStackCount` _returnvalue_2 (struct :`TagName` "GameplayTagStack.Arcade.Active.HellfireNova.DamageInterval.Enable")))) (`VyraAbilitySystemComponent.GetGameplayTagStackCount` _returnvalue_2 (struct :`TagName` "GameplayTagStack.Arcade.Active.HellfireNova.DamageInterval")) (`self.MakeOutgoingGameplayEffectSpec` (`self.GetDamageGameplayEffectClass`) 5.0) null))

(event `self.OnNormalChannelling`
  (params (TotalChannelTime :type "Float (single-precision)"))
  (bind _returnvalue (`VyraBlueprintFunctionLibrary.GetVyraAbilitySystemComponent`))
  (bind _returnvalue_2 (`self.GetAvatarActorFromActorInfo`))
  (`parent.OnNormalChannelling` TotalChannelTime)
  (`|SpawnActorFromClass` "/Game/AbilitySystem/Abilities/Arcade/Active/HellfireNova/B_HellfireNova_Collider.B_HellfireNova_Collider_C" (`Actor.GetTransform` _returnvalue_2) "AlwaysSpawn" "MultiplyWithRoot" _returnvalue_2 1.0 (`VyraAbilitySystemComponent.GetGameplayTagStackCount` _returnvalue (struct :`TagName` "GameplayTagStack.Arcade.Active.HellfireNova.MaxRadius")) 5.0 (`KismetMathLibrary.Conv_IntToBool` (`KismetMathLibrary.FFloor` (`VyraAbilitySystemComponent.GetGameplayTagStackCount` _returnvalue (struct :`TagName` "GameplayTagStack.Arcade.Active.HellfireNova.DamageInterval.Enable")))) (`VyraAbilitySystemComponent.GetGameplayTagStackCount` _returnvalue (struct :`TagName` "GameplayTagStack.Arcade.Active.HellfireNova.DamageInterval")) (`self.MakeOutgoingGameplayEffectSpec` (`self.GetDamageGameplayEffectClass`)) null))