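; Arcade Firestorm gameplay ability: a cast-time area damage spell placed at a targeted location.
; Activation takes instant target data from a Firestorm target actor, then plays a montage scaled by cast speed.
; Casting start spawns the damage actor and a ghost visual there; success starts the damage event and removes the ghost.
; Montage interruption or cancellation notifies the damage actor, broadcasts a cast-failed UI message and removes the ghost.
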(event `self.OnCastingStarted`
  (`parent.OnCastingStarted`)
  (bind _returnvalue (`|SpawnActorFromClass` "/Game/AbilitySystem/Abilities/Arcade/Active/Firestorm/B_Firestorm_Actor.B_Firestorm_Actor_C" (`AbilitySystemBlueprintLibrary.GetTargetDataEndPointTransform` (`self.TargetData`)) "AlwaysSpawn" "MultiplyWithRoot" (`self.GetAvatarActorFromActorInfo`) self 500.0 3.0 (`self.GE_Damage`) 0.95 null))
  (set `self.FirestormDamageActor` _returnvalue)
  (bind _returnvalue_2 (`|SpawnActorFromClass` "/Game/AbilitySystem/Abilities/Arcade/Active/Firestorm/B_Firestorm_TargetActor_Ghost.B_Firestorm_TargetActor_Ghost_C" (`AbilitySystemBlueprintLibrary.GetTargetDataEndPointTransform` (`self.TargetData`)) "Undefined" "MultiplyWithRoot" null null))
  (set `self.VisActor` _returnvalue_2))

(event `self.OnCastingSucceeded`
  (`parent.OnCastingSucceeded`)
  (`Firestorm_DamageActor.StartDamageEvent` (`self.FirestormDamageActor`))
  (`self.K2_EndAbility`)
  (bind _visactor (`self.VisActor`)
    (:`then`
      (`Actor.K2_DestroyActor` _visactor))
    (:`else`)))

(event `self.K2_ActivateAbility`
  (bind (_asynctaskproxy _data) (`AbilityTask_WaitTargetData.WaitTargetData` "None" "Instant" "/Game/AbilitySystem/Abilities/Arcade/Active/Firestorm/B_Firestorm_TargetActor.B_Firestorm_TargetActor_C" 500.0 (struct :`Name` "BlockAll") true (`self.MakeTargetLocationInfoFromOwnerActor`) (struct) null (struct) true)
    (:`ValidData`
      (set `self.TargetData` _data)
      (`GSCTask_PlayMontageWaitForEvent.PlayMontageAndWaitForEvent` "None" (`self.MontageToPlay`) (struct) (`self.GetCastSpeed`)
        (:`then`
          (`parent.K2_ActivateAbility`))
        (:`OnCompleted`
          (`self.K2_EndAbility` :!label _label))
        (:`OnBlendOut`
          (goto _label))
        (:`OnInterrupted`
          (`self.K2_EndAbility` :!label _label_2)
          (`Firestorm_DamageActor.AbilityCastFailed` (`self.FirestormDamageActor`))
          (`GameplayMessageSubsystem.K2_BroadcastMessage` (subsystem `GameplayMessageSubsystem`) (struct :`TagName` "UIMessaging.Ability.Cast.Failed") (make `VyraCastTimeMessage` "" 1.0))
          (bind _visactor (`self.VisActor`)
            (:`then`
              (`Actor.K2_DestroyActor` _visactor))
            (:`else`)))
        (:`OnCancelled`
          (goto _label_2))))
    (:`Cancelled`
      (`self.K2_EndAbility`))))