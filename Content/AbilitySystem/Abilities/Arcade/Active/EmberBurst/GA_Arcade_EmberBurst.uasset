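; GA_Arcade_EmberBurst is an active Arcade ability that fires a cone of ember projectiles after a cast.
; Cast start plays a montage at cast speed, ending the ability when it finishes, or also broadcasting a cast-failed UI message if interrupted or cancelled.
; A successful cast spawns the projectiles, widening the cone half-angle as the projectile count rises.
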(event `self.K2_ActivateAbility`
  (`parent.K2_ActivateAbility`))

(event `self.OnCastingStarted`
  (`parent.OnCastingStarted`)
  (`GSCTask_PlayMontageWaitForEvent.PlayMontageAndWaitForEvent` "None" (`self.MontageToPlay`) (struct) (`self.GetCastSpeed`)
    (:`OnCompleted`
      (`self.K2_EndAbility` :!label _label))
    (:`OnBlendOut`
      (goto _label))
    (:`OnInterrupted`
      (`self.K2_EndAbility` :!label _label_2)
      (`GameplayMessageSubsystem.K2_BroadcastMessage` (subsystem `GameplayMessageSubsystem`) (struct :`TagName` "UIMessaging.Ability.Cast.Failed") (make `VyraCastTimeMessage` "" 1.0)))
    (:`OnCancelled`
      (goto _label_2))))

(event `self.OnCastingSucceeded`
  (bind _returnvalue (`self.GetProjectileCount`))
  (`parent.OnCastingSucceeded`)
  (`self.SpawnProjectilesInCone` _returnvalue (`KismetMathLibrary.MapRangeClamped` (`KismetMathLibrary.Conv_IntToDouble` _returnvalue) 1.0 10.0 5.0 30.0)))