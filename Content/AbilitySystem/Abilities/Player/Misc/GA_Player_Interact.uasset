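; Player gameplay ability that detects nearby interactable objects and triggers interaction with them on input.
; A single-line trace task scans from the owning actor; when results change, it disables the previous targets' interact UI, stores the new options and updates interactions.
; A self-rearming input-press wait triggers the interaction and sends it an interact event with the avatar as instigator.
; Debug prints mark when the ability activates and ends.
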(event `self.K2_ActivateAbility`
  (`KismetSystemLibrary.PrintString` "Interaction Available")
  (`self.LookForInteractables`)
  (`self.Interact_PressScan`))

(event `self.K2_OnEndAbility`
  (params (bWasCancelled :type Boolean))
  (`KismetSystemLibrary.PrintString` "Interaction Unavailable"))

(event `LookForInteractables`
  (bind (_asynctaskproxy _interactableoptions) (`AbilityTask_WaitForInteractableTargets_SingleLineTrace.WaitForInteractableTargets_SingleLineTrace` (make `InteractionQuery` (`self.GetAvatarActorFromActorInfo`) (cast `Controller` (`self.GetOwningActorFromActorInfo`) :!pure true)) (struct :`Name` "Interactable_BlockDynamic") (`self.MakeTargetLocationInfoFromOwnerActor`) 200.0)
    (:`InteractableObjectsChanged`
      ;[0.02519 0.02217 0.02029] Disable previous interaction widgets
      (for _array_element (`self.CurrentInteractions`)
        (message `InteractionInfoAndActions.DisableInteractUI` (`KismetSystemLibrary.Conv_InterfaceToObject` (`.InteractableTarget` (break `InteractionOption` _array_element)))))
      (bind _output_get (set `self.CurrentInteractions` _interactableoptions))
      (`self.UpdateInteractions` _output_get))))

(event `Interact_PressScan`
  (`AbilityTask_WaitInputPress.WaitInputPress` false
    (:`OnPress`
      (`|ExecutionSequence`
        (:`then_0`
          (bind _returnvalue (`self.TriggerInteraction`))
          (message `InteractionInfoAndActions.OnInteractEvent` _returnvalue (make `GameplayEventData` (struct) (`self.GetAvatarActorFromActorInfo`))))
        (:`then_1`
          (`self.Interact_PressScan`))))))