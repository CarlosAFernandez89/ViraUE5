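; Player jump gameplay ability that triggers the character's jump and its animation.
; On activation it starts a WaitInputRelease task, jumps the Vyra anim instance to a named jump node, and calls Jump on the character if CanJump passes.
; Releasing the input or ending the ability calls StopJumping, so the jump follows how long the button is held.
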(event `self.K2_ActivateAbility`
  (bind _returnvalue (`self.GetVyraPlayerStateCharacter`))
  (`parent.K2_ActivateAbility`)
  (bind _asynctaskproxy (`AbilityTask_WaitInputRelease.WaitInputRelease` true)
    (:`then`
      (set `self.WaitJump_Async` _asynctaskproxy)
      (`PaperZDAnimInstance.JumpToNode` (`self.GetVyraAnimInstance`) (`self.AnimInstanceJumpNodeName`) "None")
      (if (`Character.CanJump` _returnvalue)
        (`Character.Jump` _returnvalue)))
    (:`OnRelease`
      (`Character.StopJumping` (`self.GetVyraPlayerStateCharacter`) :!label _label))))

(event `self.K2_OnEndAbility`
  (params (bWasCancelled :type Boolean))
  (`parent.K2_OnEndAbility` bWasCancelled)
  (goto _label))