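; Player movement Gameplay Ability that provides a coyote jump, accepting a jump press within a short grace period.
; On activation it listens for a fresh input press and starts a timer lasting CoyoteJumpDuration.
; A press calls ActivateCoyoteJump and prints a debug message.
; Ending the ability clears and invalidates the timer handle.
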(event `self.K2_ActivateAbility`
  (`parent.K2_ActivateAbility`)
  (`AbilityTask_WaitInputPress.WaitInputPress` false
    (:`then`
      (bind _returnvalue (`KismetSystemLibrary.K2_SetTimerDelegate` (`|CreateDelegate` :!event `K2_EndAbility`) (`self.CoyoteJumpDuration`)))
      (set `self.CoyoteTimeEnd_Timer` _returnvalue))
    (:`OnPress`
      (`self.ActivateCoyoteJump`)
      (`KismetSystemLibrary.PrintText` "Coyote Jump"))))

(event `self.K2_OnEndAbility`
  (params (bWasCancelled :type Boolean))
  (`parent.K2_OnEndAbility` bWasCancelled)
  (`KismetSystemLibrary.K2_ClearAndInvalidateTimerHandle` (`self.CoyoteTimeEnd_Timer`)))