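; Player dash gameplay ability that plays a montage while letting the character phase through collision.
; On activation it starts the montage, caches the capsule's collision profile and switches it to VyraPhasingPawn.
; Montage completion, blend-out, interruption or cancellation ends the ability, which restores the cached profile and prints a debug message.
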(event `self.K2_ActivateAbility`
  (bind _capsulecomponent (`Character.CapsuleComponent` (`self.GetVyraPlayerStateCharacter`)))
  (`parent.K2_ActivateAbility`)
  (`GSCTask_PlayMontageWaitForEvent.PlayMontageAndWaitForEvent` "None" (`self.MontageToPlay`) (struct) 1.0 "None" false
    (:`then`
      (set `self.CollisionProfileName` (`PrimitiveComponent.GetCollisionProfileName` _capsulecomponent))
      (`PrimitiveComponent.SetCollisionProfileName` _capsulecomponent "VyraPhasingPawn" false))
    (:`OnCompleted`
      (`self.K2_EndAbility` :!label _label))
    (:`OnBlendOut`
      (goto _label))
    (:`OnInterrupted`
      (goto _label))
    (:`OnCancelled`
      (goto _label))))

(event `self.K2_OnEndAbility`
  (params (bWasCancelled :type Boolean))
  (`parent.K2_OnEndAbility` bWasCancelled)
  (`KismetSystemLibrary.PrintString` "Ability Ended..")
  (`PrimitiveComponent.SetCollisionProfileName` (`Character.CapsuleComponent` (`self.GetVyraPlayerStateCharacter`)) (`self.CollisionProfileName`) false))