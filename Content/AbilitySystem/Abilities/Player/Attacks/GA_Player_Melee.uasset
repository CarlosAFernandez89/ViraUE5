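; Player melee gameplay ability that plays a horizontal, up or down attack animation from move input, at an attribute-driven rate.
; The down attack also halves the character's velocity.
; A one-shot collision event applies damage, launches hit characters away, scaled down by a target attribute, and broadcasts an EmberHeart burn message.
; Each applied damage effect grants mana and broadcasts BloodFrenzy; ability end sets gravity scale to a fixed value.
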(event `self.K2_ActivateAbility`
  (bind (_bsuccessfullyfoundattribute _returnvalue) (`AbilitySystemBlueprintLibrary.GetFloatAttribute` (`self.GetAvatarActorFromActorInfo`) (struct :`AttributeName` "AttackSpeed" :`Attribute` "/Script/Vira.CombatAttributeSet:AttackSpeed" :`AttributeOwner` "/Script/CoreUObject.Class'/Script/Vira.CombatAttributeSet'")))
  (bind _charactermovement (`Character.CharacterMovement` (`self.GetVyraPlayerStateCharacter`)))
  (bind (_velocity_x _velocity_y _velocity_z) (`KismetMathLibrary.BreakVector` (`MovementComponent.Velocity` _charactermovement)))
  (`parent.K2_ActivateAbility`)
  (bind (_asynctaskproxy _payload) (`AbilityAsync_WaitGameplayEvent.WaitGameplayEventToActor` (`self.GetVyraPlayerStateCharacter`) (struct :`TagName` "Event.Combat.Attack.Collision") true)
    (:`then`
      (bind _returnvalue_2 (message `PlayerInputHelper.GetIAMoveValue` (`self.GetVyraPlayerStateCharacter`)))
      (switch `EAttackDirection` (`self.GetAttackDirection` _returnvalue_2)
        (:`Horizontal`
          (bind _horizontalattackanim (`self.HorizontalAttackAnim`)
            (:`then`
              (`PaperZDPlaySlotOverrideAction.PlayAnimationOverrideWithCallbacks` (`self.GetVyraAnimInstance`) _horizontalattackanim "DefaultSlot" _returnvalue
                (:`OnCompleted`
                  _)
                (:`OnCancelled`
                  _)))
            (:`else`
              _))
          (`self.K2_EndAbility`))
        (:`Up`
          (bind _upattackanim (`self.UpAttackAnim`)
            (:`then`
              (`PaperZDPlaySlotOverrideAction.PlayAnimationOverrideWithCallbacks` (`self.GetVyraAnimInstance`) _upattackanim "DefaultSlot" _returnvalue
                (:`OnCompleted`
                  _)
                (:`OnCancelled`
                  _)))
            (:`else`
              _))
          (`self.K2_EndAbility`))
        (:`Down`
          (bind _downattackanim (`self.DownAttackAnim`)
            (:`then`
              (`PaperZDPlaySlotOverrideAction.PlayAnimationOverrideWithCallbacks` (`self.GetVyraAnimInstance`) _downattackanim "DefaultSlot" _returnvalue
                (:`then`
                  (set `MovementComponent.Velocity` (`KismetMathLibrary.MakeVector` (* _velocity_x 0.5) (* _velocity_y 0.5) (* _velocity_z 0.5)) _charactermovement))
                (:`OnCompleted`
                  (`self.K2_EndAbility` :!label _label))
                (:`OnCancelled`
                  (goto _label))))
            (:`else`
              (goto _label))))))
    (:`EventReceived`
      (`|ExecutionSequence`
        (:`then_0`
          (bind (_eventtag _instigator _target _optionalobject _optionalobject2 _contexthandle _instigatortags _targettags _eventmagnitude _targetdata) (break `GameplayEventData` _payload))
          (bind _returnvalue_3 (`self.BP_ApplyGameplayEffectToTarget` _targetdata (`self.GE_Damage`)))
          (for _ _returnvalue_3
            (`self.ApplyOnHitEffect`)))
        (:`then_1`
          (`self.ApplyKnockback` _targetdata))
        (:`then_2`
          (`GameplayMessageSubsystem.K2_BroadcastMessage` (subsystem `GameplayMessageSubsystem`) (struct :`TagName` "GameplayAbilityEvent.EmberHeart.Burn") _targetdata))))))

(event `self.K2_OnEndAbility`
  (params (bWasCancelled :type Boolean))
  (`parent.K2_OnEndAbility` bWasCancelled)
  (set `CharacterMovementComponent.GravityScale` 1.35 (`Character.CharacterMovement` (`self.GetVyraPlayerStateCharacter`))))

(event `ApplyOnHitEffect`
  (`self.BP_ApplyGameplayEffectToOwner` "/Game/AbilitySystem/Abilities/Player/Attacks/GE_Player_Melee_ManaRegain.GE_Player_Melee_ManaRegain_C")
  (`GameplayMessageSubsystem.K2_BroadcastMessage` (subsystem `GameplayMessageSubsystem`) (struct :`TagName` "GameplayAbilityEvent.BloodFrenzy") (`Actor.GetTransform` (`self.GetAvatarActorFromActorInfo`))))

(fn `ApplyKnockback`
  (params (TargetData :type "GameplayAbilityTargetDataHandle Structure"))
  (for _array_element (`AbilitySystemBlueprintLibrary.GetActorsFromTargetData` TargetData)
    (bind _ascharacter (cast `Character` _array_element))
    (bind (_bsuccessfullyfoundattribute _returnvalue) (`AbilitySystemBlueprintLibrary.GetFloatAttributeBaseFromAbilitySystemComponent` (`AbilitySystemBlueprintLibrary.GetAbilitySystemComponent` _ascharacter) (struct :`AttributeName` "KnockBackResistance" :`Attribute` "/Script/Vira.CombatAttributeSet:KnockBackResistance" :`AttributeOwner` "/Script/CoreUObject.Class'/Script/Vira.CombatAttributeSet'")))
    (`Character.LaunchCharacter` _ascharacter (* (`KismetMathLibrary.Normal` (- (`Actor.K2_GetActorLocation` _array_element) (`Actor.K2_GetActorLocation` (`self.GetVyraPlayerStateCharacter`)))) (* (`self.KnockBackStrength`) (- 1.0 (`KismetMathLibrary.SelectFloat` _returnvalue 0.0 _bsuccessfullyfoundattribute)))) true false)))