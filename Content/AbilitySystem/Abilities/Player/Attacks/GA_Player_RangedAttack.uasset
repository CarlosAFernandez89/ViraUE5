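; Player ranged attack ability that plays an animation and fires a damaging projectile.
; A gameplay event, awaited on the player character, spawns the projectile just ahead along the avatar's facing, while animation completion or cancellation ends the ability.
; The PenetratingFire charm tag enables phasing, so hits broadcast an EmbersEcho hit message instead of destroying the projectile.
; The destruction broadcast's binding is disconnected.
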(event `self.K2_ActivateAbility`
  (`parent.K2_ActivateAbility`)
  (`AbilityAsync_WaitGameplayEvent.WaitGameplayEventToActor` (`self.GetVyraPlayerStateCharacter`) (struct :`TagName` "Event.Combat.Attack.Ranged") true
    (:`then`
      (`self.FireAttack`))
    (:`EventReceived`
      (`self.OnSpawnProjectile`))))

(event `FireAttack`
  (`PaperZDPlaySlotOverrideAction.PlayAnimationOverrideWithCallbacks` (`self.GetVyraAnimInstance`) (`self.HorizontalAttackAnim`)
    (:`OnCompleted`
      _)
    (:`OnCancelled`
      _))
  (`self.K2_EndAbility`))

(event `OnSpawnProjectile`
  (bind _returnvalue (`self.GetAvatarActorFromActorInfo`))
  (bind _returnvalue_2 (`self.GetAvatarActorFromActorInfo`))
  (bind _returnvalue_3 (`Actor.GetActorForwardVector` _returnvalue))
  (bind _returnvalue_4 (`|SpawnActorFromClass` (`self.ProjectileClass`) (`KismetMathLibrary.MakeTransform` (+ (`Actor.K2_GetActorLocation` _returnvalue_2) (* _returnvalue_3 15.0)) (`KismetMathLibrary.MakeRotFromX` _returnvalue_3)) "AdjustIfPossibleButAlwaysSpawn" "MultiplyWithRoot" _returnvalue_2 (`self.GE Damage`) (`self.ExtraDamage`) (`GSCBlueprintFunctionLibrary.HasMatchingGameplayTag` _returnvalue (struct :`TagName` "CharmAbility.PenetratingFire")) null))
  (`/Engine/EditorBlueprintResources/StandardMacros.IsValid` _returnvalue_4
    (:`Is Valid`
      (add `/Game/AbilitySystem/Abilities/Player/Attacks/B_RangedAttack_Projectile.OnCollideWithTarget` _returnvalue_4 (`|CreateDelegate` :!event `OnProjectileHitTarget`)))))

(event `OnProjectileHitTarget`
  (params (ProjectileReference :type "Actor Object Reference"))
  (if (not (`GSCBlueprintFunctionLibrary.HasMatchingGameplayTag` (`self.GetAvatarActorFromActorInfo`) (struct :`TagName` "CharmAbility.PenetratingFire")))
    (`Actor.K2_DestroyActor` ProjectileReference)
    (else
      (`GameplayMessageSubsystem.K2_BroadcastMessage` (subsystem `GameplayMessageSubsystem`) (struct :`TagName` "CharmAbility.EmbersEcho.Hit") (`Actor.GetTransform` ProjectileReference)))))

(event `OnProjectileDestroyed`
  (params (DestroyedActor :type "Actor Object Reference"))
  (`GameplayMessageSubsystem.K2_BroadcastMessage` (subsystem `GameplayMessageSubsystem`) (struct :`TagName` "CharmAbility.EmbersEcho") (`Actor.GetTransform` DestroyedActor)))